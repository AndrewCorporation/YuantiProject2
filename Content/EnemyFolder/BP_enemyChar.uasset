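; Enemy character that patrols points, chases the player on sight and teleports them to a set location when caught.
; Patrol loops through PatrolPoints with AI MoveTo and a pause, until PawnSensing spots ThirdPersonCharacter_Paco.
; Tick then drives the chase and, at close range, the "attack" teleport, which clears the seen flag.
; CambiarState feeds the ABP_Enemygo animation state, while MakeDMG only subtracts and prints health, with no death handling.
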(event OnSeePawn(PawnSensing)
  (params (Pawn :type Pawn%20Object%20Reference))
  (bind _asthird_person_character_paco (Utilities|Casting|CastToThirdPersonCharacter_Paco Pawn))
  (Variables|Default|SetPlayerRef _asthird_person_character_paco)
  (Variables|Default|SetPlayerVisto true))

(event Custom|PatroltoPoint
  (if (not (Variables|Default|GetPlayerVisto))
    (CallFunction|CambiarState 1)
    (AI|AIMoveTo self "0, 0, 0" (Utilities|Array|Get(acopy) (Variables|Default|GetPatrolPoints) (Variables|Default|GetPoint_Index)) 5.0 false
      (:OnSuccess
        (if (>= (Variables|Default|GetPoint_Index) (- (Utilities|Array|Length (Variables|Default|GetPatrolPoints)) 1))
          (Variables|Default|SetPoint_Index 0)
          (else
            (Math|Integer|IncrementInt (Variables|Default|GetPoint_Index)
              (:%20%20
                _))))
        (CallFunction|CambiarState)
        (Utilities|FlowControl|Delay 2.0)
        (CallFunction|PatroltoPoint)))))

(event Custom|AtacarPlayer
  (CallFunction|CambiarState 2)
  (Transformation|SetActorLocation (Variables|Default|GetPlayerRef) (Transformation|GetActorLocation (Variables|Default|GetlocationPlayer)) false false)
  (Variables|Default|SetPlayerVisto false))

(event Custom|SeguirPlayer
  (CallFunction|CambiarState 2)
  (AI|AIMoveTo self "0, 0, 0" (Variables|Default|GetPlayerRef) 35.0 false))

(event EventBeginPlay
  (if (not (Variables|Default|GetPlayerVisto))
    (CallFunction|PatroltoPoint)))

(event EventTick
  (params (DeltaSeconds :type Float%20%28single-precision%29))
  (if (Variables|Default|GetPlayerVisto)
    (CallFunction|SeguirPlayer)
    (Variables|Default|Setdistancia (Transformation|GetDistanceTo (Variables|Default|GetPlayerRef)))
    (if (<= (Variables|Default|Getdistancia) 9e+01)
      (CallFunction|AtacarPlayer)
      (else
        (CallFunction|CambiarState 1)))))

(fn ConstructionScript)

(fn MakeDMG
  (params (playerDMG :type Float%20%28single-precision%29))
  (bind _output_get (Variables|Default|SetEnemyHealth (- (Variables|Default|GetEnemyHealth) playerDMG)))
  (Development|PrintString (Utilities|String|ToString(Float) _output_get) true true "(R=0.640625,G=0.100098,B=0.162988,A=1.000000)"))

(fn CambiarState
  (params (Estado :type Integer))
  (bind _asabp_enemygo (Utilities|Casting|CastToABP_Enemygo (Components|SkeletalMesh|GetAnimInstance (Variables|Character|GetMesh))))
  (switch int Estado
    (:Default
      (Variables|/Game/EnemyFolder/Modelos/Animaciones/ABP_Enemygo.ABP_Enemygo_C|SetStadosAnim _asabp_enemygo 0 :!label _label))
    (:0
      (goto _label))
    (:1
      (Variables|/Game/EnemyFolder/Modelos/Animaciones/ABP_Enemygo.ABP_Enemygo_C|SetStadosAnim _asabp_enemygo 1))
    (:2
      (Variables|/Game/EnemyFolder/Modelos/Animaciones/ABP_Enemygo.ABP_Enemygo_C|SetStadosAnim _asabp_enemygo 2))))